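; Anim notify state that lets the BP_Nanana character keep rotating during the part of a root motion animation it spans.
; On begin it casts the mesh owner to BP_Nanana and enables AllowPhysicsRotationDuringAnimRootMotion on its CharacterMovement.
; On end it sets the flag back to false rather than restoring the previous value; other owners are ignored.
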(fn `Received_NotifyBegin`
  (params (MeshComp :type "SkeletalMeshComponent Object Reference") (Animation :type "AnimSequenceBase Object Reference") (TotalDuration :type "Float (double-precision)"))
  (returns (ReturnValue :type Boolean))
  (bind _asbp_nanana (cast `/Game/IronFistGirl/Blueprints/BP_Nanana` (`ActorComponent.GetOwner` MeshComp)))
  (bind _output_get (set `CharacterMovementComponent.bAllowPhysicsRotationDuringAnimRootMotion` true (`Character.CharacterMovement` _asbp_nanana)))
  (return _output_get))

(fn `Received_NotifyEnd`
  (params (MeshComp :type "SkeletalMeshComponent Object Reference") (Animation :type "AnimSequenceBase Object Reference"))
  (returns (ReturnValue :type Boolean))
  (bind _asbp_nanana (cast `/Game/IronFistGirl/Blueprints/BP_Nanana` (`ActorComponent.GetOwner` MeshComp)))
  (bind _output_get (set `CharacterMovementComponent.bAllowPhysicsRotationDuringAnimRootMotion` false (`Character.CharacterMovement` _asbp_nanana)))
  (return _output_get))
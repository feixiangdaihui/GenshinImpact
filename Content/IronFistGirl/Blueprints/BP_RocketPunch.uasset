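; BP_RocketPunch is a rocket-punch projectile that explodes on impact.
; It keeps collision off briefly after spawning, then on hit ignores any actor that has a valid owner.
; Physics-simulating components receive an impulse scaled from the punch's velocity, while anything else takes damage.
; Both cases spawn an explosion at the hit point, then after a delay a second at the projectile's location before destroying it.
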(event `self.ReceiveBeginPlay`
  (`self.SetActorEnableCollision` false)
  (`KismetSystemLibrary.Delay` 0.05)
  (`self.SetActorEnableCollision` true))

(event `self.ReceiveHit`
  (params (MyComp :type "PrimitiveComponent Object Reference") (Other :type "Actor Object Reference") (OtherComp :type "PrimitiveComponent Object Reference") (bSelfMoved :type Boolean) (HitLocation :type "Vector Structure") (HitNormal :type "Vector Structure") (NormalImpulse :type "Vector Structure") (Hit :type "HitResult Structure (by ref)"))
  (if (`KismetSystemLibrary.IsValid` (`self.GetOwner` Other))
    _
    (elif (`SceneComponent.IsSimulatingPhysics` OtherComp "None")
      (`GameplayStatics.SpawnEmitterAtLocation` "/Game/IronFistGirl/Niagara/Particles/P_Explosion.P_Explosion" HitLocation (struct) (2.0 2.0 2.0))
      (`PrimitiveComponent.AddImpulseAtLocation` OtherComp (* (`self.GetVelocity`) 100.0) HitLocation "None")
      (`KismetSystemLibrary.Delay` 2.0)
      (`GameplayStatics.SpawnEmitterAtLocation` "/Game/IronFistGirl/Niagara/Particles/P_Explosion.P_Explosion" (`self.K2_GetActorLocation`) (struct) (2.0 2.0 2.0))
      (`self.K2_DestroyActor`)
      (else
        (`GameplayStatics.SpawnEmitterAtLocation` "/Game/IronFistGirl/Niagara/Particles/P_Explosion.P_Explosion" HitLocation (struct) (2.0 2.0 2.0))
        (`GameplayStatics.ApplyDamage` Other 200.0)
        (`KismetSystemLibrary.Delay` 2.0)
        (`GameplayStatics.SpawnEmitterAtLocation` "/Game/IronFistGirl/Niagara/Particles/P_Explosion.P_Explosion" (`self.K2_GetActorLocation`) (struct) (2.0 2.0 2.0))
        (`self.K2_DestroyActor`)))))

(fn `UserConstructionScript`)
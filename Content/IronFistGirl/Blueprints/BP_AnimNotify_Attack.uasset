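; Anim notify state that opens melee hit windows during BP_Nanana's attack animations.
; On begin it casts the mesh owner to BP_Nanana and sets each hand and foot hit component to query-and-physics or no collision, based on per-limb bool flags.
; On end it disables collision on all four, so the chosen limbs collide only within the notify's span.
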(fn `Received_NotifyBegin`
  (params (MeshComp :type "SkeletalMeshComponent Object Reference") (Animation :type "AnimSequenceBase Object Reference") (TotalDuration :type "Float (double-precision)"))
  (returns (ReturnValue :type Boolean))
  (bind _asbp_nanana (cast `/Game/IronFistGirl/Blueprints/BP_Nanana` (`ActorComponent.GetOwner` MeshComp)))
  (`PrimitiveComponent.SetCollisionEnabled` (`/Game/IronFistGirl/Blueprints/BP_Nanana.Hit_LeftFoot` _asbp_nanana) (select `bool` (`self.UseCollisionLF`) :`false` "NoCollision" :`true` "QueryAndPhysics" :!type "ECollisionEnabled Enum"))
  (`PrimitiveComponent.SetCollisionEnabled` (`/Game/IronFistGirl/Blueprints/BP_Nanana.Hit_RightFoot` _asbp_nanana) (select `bool` (`self.UseCollisionRF`) :`false` "NoCollision" :`true` "QueryAndPhysics" :!type "ECollisionEnabled Enum"))
  (`PrimitiveComponent.SetCollisionEnabled` (`/Game/IronFistGirl/Blueprints/BP_Nanana.Hit_RightHand` _asbp_nanana) (select `bool` (`self.UseCollisionRH`) :`false` "NoCollision" :`true` "QueryAndPhysics" :!type "ECollisionEnabled Enum"))
  (`PrimitiveComponent.SetCollisionEnabled` (`/Game/IronFistGirl/Blueprints/BP_Nanana.Hit_LeftHand` _asbp_nanana) (select `bool` (`self.UseCollisionLH`) :`false` "NoCollision" :`true` "QueryAndPhysics" :!type "ECollisionEnabled Enum"))
  (return false))

(fn `Received_NotifyEnd`
  (params (MeshComp :type "SkeletalMeshComponent Object Reference") (Animation :type "AnimSequenceBase Object Reference"))
  (returns (ReturnValue :type Boolean))
  (bind _asbp_nanana (cast `/Game/IronFistGirl/Blueprints/BP_Nanana` (`ActorComponent.GetOwner` MeshComp)))
  (`PrimitiveComponent.SetCollisionEnabled` (`/Game/IronFistGirl/Blueprints/BP_Nanana.Hit_LeftFoot` _asbp_nanana) "NoCollision")
  (`PrimitiveComponent.SetCollisionEnabled` (`/Game/IronFistGirl/Blueprints/BP_Nanana.Hit_RightFoot` _asbp_nanana) "NoCollision")
  (`PrimitiveComponent.SetCollisionEnabled` (`/Game/IronFistGirl/Blueprints/BP_Nanana.Hit_RightHand` _asbp_nanana) "NoCollision")
  (`PrimitiveComponent.SetCollisionEnabled` (`/Game/IronFistGirl/Blueprints/BP_Nanana.Hit_LeftHand` _asbp_nanana) "NoCollision")
  (return false))
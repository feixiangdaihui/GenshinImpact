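; BP_SandBag is a damageable skeletal-mesh target that shows physical hit reactions and goes ragdoll when its life runs out.
; Hits from BP_Nanana record the struck bone; damage lowers Life and, except for the pelvis, starts a blend timeline and delayed camera-forward impulse.
; Tick simulates physics below that bone while the blend weight is positive, giving a partial-ragdoll flinch.
; A looping timer checks Life and triggers full-physics death.
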(event `self.ReceiveTick`
  (params (DeltaSeconds :type "Float (single-precision)"))
  (bind _mesh (`self.Mesh`))
  (bind _bonename (`self.BoneName`))
  (if (> (`self.BlendWeight`) 0.0)
    (`SkeletalMeshComponent.SetAllBodiesBelowSimulatePhysics` _mesh _bonename true true)
    (`SkeletalMeshComponent.SetAllBodiesBelowPhysicsBlendWeight` _mesh _bonename 0.0 false true)))

(event `HItReaction`
  (params (Bone :type Name))
  (bind _mesh (`self.Mesh`))
  (if (!= Bone "pelvis")
    (if (`self.IsHIt`)
      (set `self.BoneName` Bone)
      (`|ExecutionSequence`
        (:`then_0`
          (bind (_direction `_新規track_0`) (`Timeline|タイムライン_0` :!via `PlayFromStart`)
            (:`Update`
              (set `self.BlendWeight` `_新規track_0`)
              (`SkeletalMeshComponent.SetAllBodiesPhysicsBlendWeight` _mesh 0.0 false)
              (`SkeletalMeshComponent.SetAllBodiesSimulatePhysics` _mesh false)
              (set `self.IsHIt` false))))
        (:`then_1`
          (`KismetSystemLibrary.Delay` 0.048)
          (`PrimitiveComponent.AddImpulse` (`self.Mesh`) (* (`KismetMathLibrary.GetForwardVector` (`self.K2_GetActorRotation` (`GameplayStatics.GetPlayerCameraManager` 0))) 1200.0) (`self.BoneName`) true))))))

(event `self.ReceiveBeginPlay`
  (`KismetSystemLibrary.K2_SetTimerDelegate` (delegate `CheckLife`) 0.25 true))

(event `CheckLife`
  (if (<= (`self.Life`) 0.0)
    (`self.Death`)))

(event `Death`
  (`PrimitiveComponent.SetSimulatePhysics` (`self.Mesh`) true)
  (set `self.Dead` true))

(event `self.ReceiveAnyDamage`
  (params (Damage :type "Float (single-precision)") (DamageType :type "DamageType Object Reference") (InstigatedBy :type "Controller Object Reference") (DamageCauser :type "Actor Object Reference"))
  (set `self.Life` (- (`self.Life`) Damage))
  (set `self.IsHIt` true)
  (`self.HItReaction` (`self.BoneName`)))

(event `self.Mesh.OnComponentHit`
  (params (HitComponent :type "PrimitiveComponent Object Reference") (OtherActor :type "Actor Object Reference") (OtherComp :type "PrimitiveComponent Object Reference") (NormalImpulse :type "Vector Structure") (Hit :type "HitResult Structure (by ref)"))
  (cast `/Game/IronFistGirl/Blueprints/BP_Nanana` OtherActor)
  (set `self.BoneName` Hit_HitBoneName))

(fn `UserConstructionScript`)
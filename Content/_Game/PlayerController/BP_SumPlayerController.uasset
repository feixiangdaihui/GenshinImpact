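; Player controller that handles inventory toggling and item pickup for the player character.
; The B key toggles the inventory widget through its inventory component.
; Each tick it scans BP_Item actors overlapping the character and sends a pickup interface message to the first eligible one.
; Items flagged NeedToPick require holding G, while others implementing BPI_PickUp are picked up automatically on overlap.
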(event `Key|B`
  (params (Key :type "Key Structure"))
  (:`Pressed`
    (`/Game/_Game/Inventory/InventoryComponent.ToggleInventoryWidget` (`self.InventoryComponent1`))))

(event `self.ReceiveTick`
  (params (DeltaSeconds :type "Float (single-precision)"))
  (for _array_element (`self.GetOverlappingActors` (`GameplayStatics.GetPlayerCharacter` 0) "/Game/_Game/Inventory/BP_Item.BP_Item_C")
    (bind (_itemstruct_name _itemstruct_isstackable _itemstruct_image _itemstruct_maxstacksize _itemstruct_isconsumable _itemstruct_changedata _itemstruct_description _itemstruct_class _itemstruct_attribute _itemstruct_category _itemstruct_hasentity _itemstruct_needtopick) (break `/Game/_Game/Inventory/ItemStruct/ItemStruct` (`/Game/_Game/Inventory/BP_Item.ItemStruct` (cast `/Game/_Game/Inventory/BP_Item` _array_element :!pure true))))
    (if _itemstruct_needtopick
      (if (`self.IsInputKeyDown` (`GameplayStatics.GetPlayerController` 0) "G")
        (message `/Game/_Game/Inventory/BPI_PickUp.Interface` _array_element self :!label _label)
        (break))
      (elif (`KismetSystemLibrary.DoesImplementInterface` _array_element "/Game/_Game/Inventory/BPI_PickUp.BPI_PickUp_C")
        (goto _label)))))

(fn `UserConstructionScript`)
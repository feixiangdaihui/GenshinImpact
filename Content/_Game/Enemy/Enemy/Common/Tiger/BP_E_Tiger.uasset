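; BP_E_Tiger is the Blueprint for the Tiger enemy, handling its health readout.
; On BeginPlay it caches its EnemyHealthComponent, creates a BP_EnemyHealthWidget bound to itself and initializes its health percent to full.
; Every Tick it polls the component to refresh CurrentHealthPercent.
; The widget is never attached or added to the viewport here, and a no-op validity check and debug print remain.
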(event `self.ReceiveBeginPlay`
  (set `self.血量组件引用` (`self.GetComponentByClass` "/Script/GenshinImpact.EnemyHealthComponent"))
  (bind _returnvalue (`|CreateWidget` "/Game/_Game/Enemy/Widget/BP_EnemyHealthWidget.BP_EnemyHealthWidget_C" null self))
  (bind _output_get (set `/Game/_Game/Enemy/Widget/BP_EnemyHealthWidget.Enemy` self _returnvalue))
  (`/Engine/EditorBlueprintResources/StandardMacros.IsValid` _output_get
    (:`Is Valid`
      _)
    (:`Is Not Valid`
      _))
  (set `self.CurrentHealthPercent` 1.0)
  (`KismetSystemLibrary.PrintString` "Hello" true false))

(event `self.ReceiveTick`
  (params (DeltaSeconds :type "Float (single-precision)"))
  (set `self.CurrentHealthPercent` (`EnemyHealthComponent.GetCurrentHealthPercent` (`self.血量组件引用`))))

(fn `UserConstructionScript`)
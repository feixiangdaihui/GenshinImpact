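; BP_GachaManager is the gacha system actor that opens the gacha screen and grants a random food, drink or weapon item.
; The M key toggles WBP_GachaUI, creating or removing the widget and switching between UI-only and game-only input.
; ExecuteGacha, with no caller in this graph, spawns the rolled item at world origin and adds it to the inventory.
; The roll spans 1 to 7, so the RoastChickenFood case at 0 never fires.
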(event `self.ReceiveBeginPlay`
  (`self.EnableInput` (`GameplayStatics.GetPlayerController` 0)))

(event `Key|M`
  (params (Key :type "Key Structure"))
  (:`Pressed`
    (`self.ToggleGacha`)))

(event `ExecuteGacha`
  (bind _returnvalue (`KismetMathLibrary.MakeTransform` (0.0 0.0 0.0)))
  (switch `int` (`KismetMathLibrary.RandomIntegerInRange` 1 7)
    (:`0`
      (bind _returnvalue_2 (`|SpawnActorFromClass` "/Game/_Game/Item/RoastChickenFood.RoastChickenFood_C" _returnvalue "Undefined" "MultiplyWithRoot" null null))
      (`/Game/_Game/Item/RoastChickenFood.AddItToInventory` _returnvalue_2))
    (:`1`
      (bind _returnvalue_3 (`|SpawnActorFromClass` "/Game/_Game/Item/CheeseFood.CheeseFood_C" _returnvalue "Undefined" "MultiplyWithRoot" null null))
      (`/Game/_Game/Item/CheeseFood.AddItToInventoty` _returnvalue_3))
    (:`2`
      (bind _returnvalue_4 (`|SpawnActorFromClass` "/Game/_Game/Item/Drink.Drink_C" _returnvalue "Undefined" "MultiplyWithRoot" null null))
      (`/Game/_Game/Item/Drink.AddItToInventory` _returnvalue_4))
    (:`3`
      (bind _returnvalue_5 (`|SpawnActorFromClass` "/Game/_Game/Item/EggFood.EggFood_C" _returnvalue "Undefined" "MultiplyWithRoot" null null))
      (`/Game/_Game/Item/EggFood.AddItToInventory` _returnvalue_5))
    (:`4`
      (bind _returnvalue_6 (`|SpawnActorFromClass` "/Game/_Game/Item/Fish.Fish_C" _returnvalue "Undefined" "MultiplyWithRoot" null null))
      (`/Game/_Game/Item/Fish.AddItToInventory` _returnvalue_6))
    (:`5`
      (bind _returnvalue_7 (`|SpawnActorFromClass` "/Game/_Game/Item/GunWeapon.GunWeapon_C" _returnvalue "Undefined" "MultiplyWithRoot" null null))
      (`/Game/_Game/Item/GunWeapon.AddItToInventory` _returnvalue_7))
    (:`6`
      (bind _returnvalue_8 (`|SpawnActorFromClass` "/Game/_Game/Item/KnifeWeapon.KnifeWeapon_C" _returnvalue "Undefined" "MultiplyWithRoot" null null))
      (`/Game/_Game/Item/KnifeWeapon.AddItToInventory` _returnvalue_8))
    (:`7`
      (bind _returnvalue_9 (`|SpawnActorFromClass` "/Game/_Game/Item/PizzaFood.PizzaFood_C" _returnvalue "Undefined" "MultiplyWithRoot" null null))
      (`/Game/_Game/Item/PizzaFood.AddItToInventory` _returnvalue_9))))

(fn `ToggleGacha`
  (bind _wbp_gachaui (`self.WBP_GachaUI`))
  (bind _wbp_gachaui_2 (`self.WBP_GachaUI`)
    (:`then`
      (`Widget.RemoveFromParent` _wbp_gachaui_2)
      (set `self.WBP_GachaUI` null)
      (`WidgetBlueprintLibrary.SetInputMode_GameOnly` (`GameplayStatics.GetPlayerController` 0)))
    (:`else`
      (bind _returnvalue (`|CreateWidget` "/Game/_Game/GachaSystem/WBP_GachaUI.WBP_GachaUI_C"))
      (set `self.WBP_GachaUI` _returnvalue)
      (`UserWidget.AddToViewport` _wbp_gachaui 0)
      (`WidgetBlueprintLibrary.SetInputMode_UIOnlyEx` (`GameplayStatics.GetPlayerController` 0) _wbp_gachaui "LockAlways"))))

(fn `UserConstructionScript`)
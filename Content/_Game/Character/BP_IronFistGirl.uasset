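; BP_IronFistGirl is the Iron Fist Girl character Blueprint, handling her normal attack and spell cast inputs.
; Each Enhanced Input action checks its own boolean gate, then plays the NormalAttack or Skill montage on the mesh.
; Both raise IsAnimForbidden and IsJudgeNormalAttack during playback and clear them only on montage completion, with no interrupt handling.
; The spell spawns through SpawnCastSpell once the Skill montage completes.
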(event `EnhancedInput|/Game/_Game/Character/Animation/IA_NormalAttack`
  (params (ActionValue :type Boolean) (ElapsedSeconds :type "Float (double-precision)") (TriggeredSeconds :type "Float (double-precision)") (InputAction :type "InputAction Object Reference" :default "/Game/_Game/Character/Animation/IA_NormalAttack.IA_NormalAttack"))
  (:`Triggered`
    (if (`self.IsNormalAttack`)
      (set `self.IsAnimForbidden` true)
      (set `self.IsJudgeNormalAttack` true)
      (`|PlayMontage` (`self.Mesh`) "/Game/IronFistGirl/Animation/AnimMontage/NormalAttack.NormalAttack"
        (:`OnCompleted`
          (set `self.IsAnimForbidden` false)
          (set `self.IsJudgeNormalAttack` false))))))

(event `EnhancedInput|/Game/_Game/Character/Animation/IA_CastSpell`
  (params (ActionValue :type Boolean) (ElapsedSeconds :type "Float (double-precision)") (TriggeredSeconds :type "Float (double-precision)") (InputAction :type "InputAction Object Reference" :default "/Game/_Game/Character/Animation/IA_CastSpell.IA_CastSpell"))
  (:`Triggered`
    (if (`self.IsCastingSpell`)
      (set `self.IsJudgeNormalAttack` true)
      (set `self.IsAnimForbidden` true)
      (`|PlayMontage` (`self.Mesh`) "/Game/IronFistGirl/Animation/RootMotions/skill.skill"
        (:`OnCompleted`
          (`self.SpawnCastSpell`)
          (set `self.IsJudgeNormalAttack` false)
          (set `self.IsAnimForbidden` false))))))

(fn `UserConstructionScript`)
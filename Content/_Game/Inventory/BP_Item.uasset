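; BP_Item is a world pickup actor that adds one unit of its item to an interactor's inventory.
; A Sphere overlap with BP_PlayCharacter shows the WBP_PressKey_F prompt, and ending the overlap removes it.
; The Interface interaction event passes the item struct to the Interactive actor's InventoryComponent through AddSlotToInventory, then clears the prompt and destroys the pickup.
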(event `self.Sphere.OnComponentBeginOverlap`
  (params (OverlappedComponent :type "PrimitiveComponent Object Reference") (OtherActor :type "Actor Object Reference") (OtherComp :type "PrimitiveComponent Object Reference") (OtherBodyIndex :type Integer) (bFromSweep :type Boolean) (SweepResult :type "HitResult Structure (by ref)"))
  (cast `/Game/_Game/Character/BP_PlayCharacter` OtherActor)
  (`/Engine/EditorBlueprintResources/StandardMacros.IsValid` (`self.WBP_PressKey_F`)
    (:`Is Valid`
      (`Widget.RemoveFromParent` (`self.WBP_PressKey_F`)))
    (:`Is Not Valid`
      _))
  (bind _returnvalue (`|CreateWidget` "/Game/_Game/Inventory/WBP_PressKey_F.WBP_PressKey_F_C"))
  (set `self.WBP_PressKey_F` _returnvalue)
  (`UserWidget.AddToViewport` (`self.WBP_PressKey_F`) 0))

(event `self.Sphere.OnComponentEndOverlap`
  (params (OverlappedComponent :type "PrimitiveComponent Object Reference") (OtherActor :type "Actor Object Reference") (OtherComp :type "PrimitiveComponent Object Reference") (OtherBodyIndex :type Integer))
  (bind _wbp_presskey_f (`self.WBP_PressKey_F`))
  (cast `/Game/_Game/Character/BP_PlayCharacter` OtherActor)
  (`/Engine/EditorBlueprintResources/StandardMacros.IsValid` _wbp_presskey_f
    (:`Is Valid`
      (`Widget.RemoveFromParent` _wbp_presskey_f))))

(event `/Game/_Game/Inventory/BPI_PickUp.Interface`
  (params (Interactive :type "Actor Object Reference"))
  (bind _wbp_presskey_f (`self.WBP_PressKey_F`))
  (`/Game/_Game/Inventory/InventoryComponent.AddSlotToInventory` (`self.GetComponentByClass` Interactive "/Game/_Game/Inventory/InventoryComponent.InventoryComponent_C") (make `/Game/_Game/Inventory/SlotStruct` (`self.ItemStruct`) 1))
  (`/Engine/EditorBlueprintResources/StandardMacros.IsValid` _wbp_presskey_f
    (:`Is Valid`
      (`Widget.RemoveFromParent` _wbp_presskey_f))
    (:`Is Not Valid`
      _))
  (`self.K2_DestroyActor`))

(fn `UserConstructionScript`)